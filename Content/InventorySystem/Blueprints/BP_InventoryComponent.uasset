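; Inventory component, attachable to the player or other actors, that stores item class and amount pairs and handles pickup, stacking and use.
; AddNewItem takes the first matching or empty slot, with no stack limit.
; The nearest item drives a pickup prompt, and its actor is destroyed once collected.
; Using a usable item decrements or removes it, rebuilds the player's UI list from class defaults and returns its effect.
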(event Custom|SetupUIRef
  (params (UI :type WBP%20UI%20Object%20Reference))
  ;[1 1 1] Only called in player's Blueprint, isn't called when component attached to other actors
  (Variables|Default|SetUIRef UI))

(event EventTick
  (params (DeltaSeconds :type Float%20%28single-precision%29)))

(event Input|KeyboardEvents|F
  (params (Key :type Key%20Structure :default "None"))
  ;[1 1 1] For Debugging, Display Items without UI
  (:Pressed
    (for _array_element (Variables|Default|GetInventoryContents)
      (if (Utilities|IsValidClass (.item _array_element))
        (Development|PrintString (Utilities|GetClassDisplayName (.item _array_element)))
        (Development|PrintString (Utilities|String|ToString(Integer) (.amount _array_element)))))))

(fn AddItematIndex
  (params (InventoryContent :type Inventory%20Content%20Structure) (Index :type Integer))
  (Utilities|Array|SetArrayElem (Variables|Default|GetInventoryContents) Index InventoryContent))

(fn AddNewItem
  (params (Item :type Inventory%20Content%20Structure))
  (LocalVariables|SetLocalItem Item)
  (bind (_array_element _array_index) (Utilities|Array|ForEachLoopwithBreak (Variables|Default|GetInventoryContents) :!label _label)
    (:LoopBody
      ;[1 1 1] Check if same item exists, if not add this item to inventory
      (if (Utilities|IsValidClass (.Item (Utilities|Struct|BreakInventoryContent _array_element)))
        ;[1 1 1] Check if same item exists, if it does add to stack (for now it doesn't have stack limit)
        (if (== (.item (LocalVariables|GetLocalItem)) (.Item (Utilities|Struct|BreakInventoryContent _array_element)))
          (CallFunction|AddtoStackatIndex (LocalVariables|GetLocalItem) _array_index)
          (LocalVariables|SetItemWasAdded true :!label _label_2)
          (goto _label Break))
        (else
          (CallFunction|AddItematIndex (LocalVariables|GetLocalItem) _array_index)
          (goto _label_2))))
    (:Completed
      ;[1 1 1] Check if this is player's inventory and ignores if not
      (Utilities|IsValid (Variables|Default|GetUIRef)
        (:Is%20Valid
          (if (LocalVariables|GetItemWasAdded)
            (CallFunction|RefreshInventoryDisplay)
            (return (LocalVariables|GetItemWasAdded))
            (else
              _)))
        (:Is%20Not%20Valid
          _))
      (return (LocalVariables|GetItemWasAdded)))))

(fn AddtoStackatIndex
  (params (Item :type Inventory%20Content%20Structure) (index :type Integer))
  (bind _inventorycontents (Variables|Default|GetInventoryContents))
  (bind _output (Utilities|Array|Get(acopy) _inventorycontents index))
  (Utilities|Array|SetArrayElem (Variables|Default|GetInventoryContents) index (Utilities|Struct|MakeInventoryContent (.item _output) (+ (.amount _output) (.Amount (Utilities|Struct|BreakInventoryContent Item))))))

(fn RefreshInventoryDisplay
  (Widget|Panel|ClearChildren (Variables|/Game/Interface/WBP_UI.WBP_UI_C|GetInventoryDisplay (Variables|Default|GetUIRef)))
  (for _array_element (Variables|Default|GetInventoryContents)
    (if (Utilities|IsValidClass (.item _array_element))
      (Default|AddItemtoDisplay (Variables|Default|GetUIRef) (.icon (Utilities|GetClassDefaults (.item _array_element))) (.name (Utilities|GetClassDefaults (.item _array_element))) (Utilities|Text|ToText(Integer) (.amount _array_element))))))

(fn SetNearestItemforPickup
  (params (Item%20Content :type Inventory%20Content%20Structure) (Interactable%20Item :type Actor%20Object%20Reference))
  (Variables|Default|SetClosestItem Item%20Content)
  (bind _output_get (Variables|Default|SetClosestItem'sActor Interactable%20Item))
  (CallFunction|ShowPickupText (Utilities|IsValid _output_get)))

(fn ShowPickupText
  (params (IsActive :type Boolean))
  (bind _uiref (Variables|Default|GetUIRef))
  (if (Math|Boolean|ANDBoolean IsActive (Utilities|IsValid (Variables|Default|GetUIRef)) (Utilities|IsValidClass (.item (Variables|Default|GetClosestItem))))
    (Variables|/Script/UMG.TextBlock|SetText (Variables|/Game/Interface/WBP_UI.WBP_UI_C|GetItemName _uiref) (.name (Utilities|GetClassDefaults (.item (Variables|Default|GetClosestItem)))))
    (Variables|/Script/UMG.Widget|SetVisibility (Variables|/Game/Interface/WBP_UI.WBP_UI_C|GetPickupText _uiref) "HitTestInvisible")
    (else
      (Variables|/Script/UMG.Widget|SetVisibility (Variables|/Game/Interface/WBP_UI.WBP_UI_C|GetPickupText (Variables|Default|GetUIRef)) "Hidden"))))

(fn PickupClosestItem
  (bind _closestitem_sactor (Variables|Default|GetClosestItem'sActor))
  (Utilities|IsValid _closestitem_sactor
    (:Is%20Valid
      (bind _success (CallFunction|AddNewItem (Variables|Default|GetClosestItem)))
      (if _success
        (Actor|DestroyActor _closestitem_sactor)))))

(fn UseItematIndex
  (params (Index :type Integer))
  (bind _inventorycontents (Variables|Default|GetInventoryContents))
  (LocalVariables|SetLocalIndex Index)
  (LocalVariables|SetLocalItemContent (Utilities|Array|Get(acopy) (Variables|Default|GetInventoryContents) (LocalVariables|GetLocalIndex)))
  (if (.isusable (Utilities|GetClassDefaults (.Item (Utilities|Struct|BreakInventoryContent (Utilities|Array|Get(acopy) (Variables|Default|GetInventoryContents) (LocalVariables|GetLocalIndex))))))
    (if (Utilities|IsValidClass (.item (LocalVariables|GetLocalItemContent)))
      (if (== (.amount (LocalVariables|GetLocalItemContent)) 1)
        (Utilities|Array|RemoveIndex _inventorycontents (LocalVariables|GetLocalIndex))
        (else
          (bind _result (Math|Integer|DecrementInt (.amount (LocalVariables|GetLocalItemContent)))
            (:%20%20
              (Utilities|Array|SetArrayElem _inventorycontents (LocalVariables|GetLocalIndex) (Utilities|Struct|MakeInventoryContent (.item (LocalVariables|GetLocalItemContent)) _result))))))
      (CallFunction|RefreshInventoryDisplay)
      (return (.itemeffect (Utilities|GetClassDefaults (.item (LocalVariables|GetLocalItemContent)))) (.effectvalue (Utilities|GetClassDefaults (.item (LocalVariables|GetLocalItemContent))))))))