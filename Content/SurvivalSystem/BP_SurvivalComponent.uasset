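; Survival component that tracks hunger and thirst, starting both at their maximum on BeginPlay.
; Each Tick drains both by delta time times a multiplier, with no lower clamp, and flags low values at a quarter of maximum.
; Restore functions add amounts capped at maximum.
; Tick also pushes values to progress bars on a UI reference supplied through SetupUIRef, dividing by a fixed 100 rather than the maximum.
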(event Custom|SetupUIRef
  (params (UIRef :type WBP%20UI%20Object%20Reference))
  (Variables|Default|SetUIRef UIRef))

(event EventTick
  (params (DeltaSeconds :type Float%20%28single-precision%29))
  (CallFunction|HungerSystem DeltaSeconds)
  (CallFunction|ThirstSystem DeltaSeconds)
  (CallFunction|UpdateVisuals))

(event EventBeginPlay
  (Variables|Default|SetHungerCurrentValue (Variables|Default|GetHungerMaxValue))
  (Variables|Default|SetThirstCurrentValue (Variables|Default|GetThirstMaxValue)))

(fn HungerSystem
  (params (Delta%20Seconds :type Float%20%28double-precision%29))
  (Variables|Default|SetHungerCurrentValue (- (Variables|Default|GetHungerCurrentValue) (* Delta%20Seconds (Variables|Default|GetHungerMultiplier))))
  (Variables|Default|SetLowHunger (<= (Variables|Default|GetHungerCurrentValue) (/ (Variables|Default|GetHungerMaxValue) 4.0))))

(fn ThirstSystem
  (params (Delta%20Seconds :type Float%20%28double-precision%29))
  (Variables|Default|SetThirstCurrentValue (- (Variables|Default|GetThirstCurrentValue) (* Delta%20Seconds (Variables|Default|GetThirstMultiplier))))
  (Variables|Default|SetLowThirst (<= (Variables|Default|GetThirstCurrentValue) (/ (Variables|Default|GetThirstMaxValue) 4.0))))

(fn RestoreThirst
  (params (RestorationAmount :type Float%20%28double-precision%29))
  (if (>= (+ (Variables|Default|GetThirstCurrentValue) RestorationAmount) (Variables|Default|GetThirstMaxValue))
    (Variables|Default|SetThirstCurrentValue (Variables|Default|GetThirstMaxValue))
    (else
      (Variables|Default|SetThirstCurrentValue (+ (Variables|Default|GetThirstCurrentValue) RestorationAmount)))))

(fn RestoreHunger
  (params (RestorationAmount :type Float%20%28double-precision%29))
  (if (>= (+ (Variables|Default|GetHungerCurrentValue) RestorationAmount) (Variables|Default|GetHungerMaxValue))
    (Variables|Default|SetHungerCurrentValue (Variables|Default|GetHungerMaxValue))
    (else
      (Variables|Default|SetHungerCurrentValue (+ (Variables|Default|GetHungerCurrentValue) RestorationAmount)))))

(fn UpdateVisuals
  (Progress|SetPercent (Variables|/Game/Interface/WBP_UI.WBP_UI_C|GetHungerBar (Variables|Default|GetUIRef)) (/ (Variables|Default|GetHungerCurrentValue) 1e+02))
  (Progress|SetPercent (Variables|/Game/Interface/WBP_UI.WBP_UI_C|GetThirstBar (Variables|Default|GetUIRef)) (/ (Variables|Default|GetThirstCurrentValue) 1e+02)))